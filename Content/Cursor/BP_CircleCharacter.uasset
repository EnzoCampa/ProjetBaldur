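; BP_CircleCharacter is a colored circle marker in the Cursor system, drawn with a cylinder mesh.
; On BeginPlay it creates a dynamic instance of M_CircleCharacter on the cylinder and sets its Color parameter to blue.
; ChangeColorAlly and ChangeColorEnnemies events recolor that instance to white for allies and red for enemies.
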(event Custom|ChangeColorEnnemies
  (Rendering|Material|SetVectorParameterValue (Variables|Default|GetMID_CircleCharacter) "Color" "(R=1.000000,G=0.015156,B=0.000000,A=1.000000)" :!class /Script/Engine.MaterialInstanceDynamic))

(event Custom|ChangeColorAlly
  (Rendering|Material|SetVectorParameterValue (Variables|Default|GetMID_CircleCharacter) "Color" "(R=1.000000,G=1.000000,B=1.000000,A=1.000000)" :!class /Script/Engine.MaterialInstanceDynamic))

(event EventBeginPlay
  (bind _returnvalue (Rendering|Material|CreateDynamicMaterialInstance (Variables|Default|GetCylinder) 0 "/Game/Cursor/M_CircleCharacter.M_CircleCharacter" "None" :!class /Script/Engine.PrimitiveComponent))
  (Variables|Default|SetMID_CircleCharacter _returnvalue)
  (Rendering|Material|SetVectorParameterValue (Variables|Default|GetMID_CircleCharacter) "Color" "(R=0.000000,G=0.425515,B=1.000000,A=1.000000)" :!class /Script/Engine.MaterialInstanceDynamic))

(fn ConstructionScript)